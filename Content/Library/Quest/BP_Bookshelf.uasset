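; Library quest bookshelf with labelled side signs and up to six book slots to fill.
; On BeginPlay it randomly destroys some slots, reports the slot count to BPI_BookshelfSlots widgets, then disables the six named slots inside that widget loop.
; OnTabletGrab re-enables surviving slots.
; Overlap by any actor with "Book" in its name disables that slot and notifies the widgets of progress.
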(event `self.ReceiveBeginPlay`
  (bind _outitem (`KismetArrayLibrary.Array_Random` (`SceneComponent.GetChildrenComponents` (`self.Book slots`) false)))
  (`self.SetSigns` (`self.LeftSign`) (`self.RightSign`))
  (for _ (range (+ (`KismetMathLibrary.RandomInteger` 6) 1))
    (cast `PrimitiveComponent` _outitem)
    (`ActorComponent.K2_DestroyComponent` _outitem))
  (bind _foundwidgets (`WidgetBlueprintLibrary.GetAllWidgetsWithInterface` "/Game/Library/Quest/BPI_BookshelfSlots.BPI_BookshelfSlots_C"))
  (for _array_element _foundwidgets
    (`KismetSystemLibrary.PrintString` "Quest 2 Updated")
    (message `/Game/Library/Quest/BPI_BookshelfSlots.UpdateSlots` _array_element (`KismetArrayLibrary.Array_Length` (`SceneComponent.GetChildrenComponents` (`self.Book slots`) false)))
    ;[1 1 1] Disable before gripping tablet
    (`|ExecutionSequence`
      (:`then_0`
        (bind _book_slot_d1 (`self.Book slot d1`)
          (:`then`
            (`self.DisableSlot` null _book_slot_d1))
          (:`else`)))
      (:`then_1`
        (bind _book_slot_d2 (`self.Book slot d2`)
          (:`then`
            (`self.DisableSlot` null _book_slot_d2))
          (:`else`)))
      (:`then_2`
        (bind _book_slot_d3 (`self.Book slot d3`)
          (:`then`
            (`self.DisableSlot` null _book_slot_d3))
          (:`else`)))
      (:`then_3`
        (bind _book_slot_d4 (`self.Book slot d4`)
          (:`then`
            (`self.DisableSlot` null _book_slot_d4))
          (:`else`)))
      (:`then_4`
        (bind _book_slot_d5 (`self.Book slot d5`)
          (:`then`
            (`self.DisableSlot` null _book_slot_d5))
          (:`else`)))
      (:`then_5`
        (bind _book_slot_d6 (`self.Book slot d6`)
          (:`then`
            (`self.DisableSlot` null _book_slot_d6))
          (:`else`))))))

(event `self.Book slot d1.OnComponentBeginOverlap`
  (params (OverlappedComponent :type "PrimitiveComponent Object Reference") (OtherActor :type "Actor Object Reference") (OtherComp :type "PrimitiveComponent Object Reference") (OtherBodyIndex :type Integer) (bFromSweep :type Boolean) (SweepResult :type "HitResult Structure (by ref)"))
  ;[1 1 1] Disable slot after placing book
  (if (`KismetStringLibrary.Contains` (`KismetSystemLibrary.GetObjectName` OtherActor) "Book")
    (`self.DisableSlot` OtherActor (`self.Book slot d1`))
    (bind _foundwidgets (`WidgetBlueprintLibrary.GetAllWidgetsWithInterface` "/Game/Library/Quest/BPI_BookshelfSlots.BPI_BookshelfSlots_C" :!label _label))
    (for _array_element _foundwidgets
      (message `/Game/Library/Quest/BPI_BookshelfSlots.UpdateSlotsDone` _array_element))))

(event `self.Book slot d4.OnComponentBeginOverlap`
  (params (OverlappedComponent :type "PrimitiveComponent Object Reference") (OtherActor :type "Actor Object Reference") (OtherComp :type "PrimitiveComponent Object Reference") (OtherBodyIndex :type Integer) (bFromSweep :type Boolean) (SweepResult :type "HitResult Structure (by ref)"))
  ;[1 1 1] Disable slot after placing book
  (if (`KismetStringLibrary.Contains` (`KismetSystemLibrary.GetObjectName` OtherActor) "Book")
    (`self.DisableSlot` OtherActor (`self.Book slot d4`))
    (goto _label)))

(event `self.Book slot d2.OnComponentBeginOverlap`
  (params (OverlappedComponent :type "PrimitiveComponent Object Reference") (OtherActor :type "Actor Object Reference") (OtherComp :type "PrimitiveComponent Object Reference") (OtherBodyIndex :type Integer) (bFromSweep :type Boolean) (SweepResult :type "HitResult Structure (by ref)"))
  ;[1 1 1] Disable slot after placing book
  (if (`KismetStringLibrary.Contains` (`KismetSystemLibrary.GetObjectName` OtherActor) "Book")
    (`self.DisableSlot` OtherActor (`self.Book slot d2`))
    (goto _label)))

(event `self.Book slot d5.OnComponentBeginOverlap`
  (params (OverlappedComponent :type "PrimitiveComponent Object Reference") (OtherActor :type "Actor Object Reference") (OtherComp :type "PrimitiveComponent Object Reference") (OtherBodyIndex :type Integer) (bFromSweep :type Boolean) (SweepResult :type "HitResult Structure (by ref)"))
  ;[1 1 1] Disable slot after placing book
  (if (`KismetStringLibrary.Contains` (`KismetSystemLibrary.GetObjectName` OtherActor) "Book")
    (`self.DisableSlot` OtherActor (`self.Book slot d5`))
    (goto _label)))

(event `/Game/Library/Quest/BPI_QuestBus.OnTabletGrab`
  ;[1 1 1] Enable slots after gripping tablet
  (`|ExecutionSequence`
    (:`then_0`
      (bind _book_slot_d1 (`self.Book slot d1`)
        (:`then`
          (`self.DisableSlot` null _book_slot_d1 true))
        (:`else`)))
    (:`then_1`
      (bind _book_slot_d2 (`self.Book slot d2`)
        (:`then`
          (`self.DisableSlot` null _book_slot_d2 true))
        (:`else`)))
    (:`then_2`
      (bind _book_slot_d3 (`self.Book slot d3`)
        (:`then`
          (`self.DisableSlot` null _book_slot_d3 true))
        (:`else`)))
    (:`then_3`
      (bind _book_slot_d4 (`self.Book slot d4`)
        (:`then`
          (`self.DisableSlot` null _book_slot_d4 true))
        (:`else`)))
    (:`then_4`
      (bind _book_slot_d5 (`self.Book slot d5`)
        (:`then`
          (`self.DisableSlot` null _book_slot_d5 true))
        (:`else`)))
    (:`then_5`
      (bind _book_slot_d6 (`self.Book slot d6`)
        (:`then`
          (`self.DisableSlot` null _book_slot_d6 true))
        (:`else`)))))

(event `self.Book slot d3.OnComponentBeginOverlap`
  (params (OverlappedComponent :type "PrimitiveComponent Object Reference") (OtherActor :type "Actor Object Reference") (OtherComp :type "PrimitiveComponent Object Reference") (OtherBodyIndex :type Integer) (bFromSweep :type Boolean) (SweepResult :type "HitResult Structure (by ref)"))
  ;[1 1 1] Disable slot after placing book
  (if (`KismetStringLibrary.Contains` (`KismetSystemLibrary.GetObjectName` OtherActor) "Book")
    (`self.DisableSlot` OtherActor (`self.Book slot d3`))
    (goto _label)))

(event `self.Book slot d6.OnComponentBeginOverlap`
  (params (OverlappedComponent :type "PrimitiveComponent Object Reference") (OtherActor :type "Actor Object Reference") (OtherComp :type "PrimitiveComponent Object Reference") (OtherBodyIndex :type Integer) (bFromSweep :type Boolean) (SweepResult :type "HitResult Structure (by ref)"))
  ;[1 1 1] Disable slot after placing book
  (if (`KismetStringLibrary.Contains` (`KismetSystemLibrary.GetObjectName` OtherActor) "Book")
    (`self.DisableSlot` OtherActor (`self.Book slot d6`))
    (goto _label)))

(fn `DisableSlot`
  (params (`Overlap object` :type "Object Object Reference") (`Slot target` :type "PrimitiveComponent Object Reference") (Enable :type Boolean))
  (bind _returnvalue (not Enable))
  (bind _returnvalue_2 (not _returnvalue))
  (`SceneComponent.SetHiddenInGame` `Slot target` _returnvalue false)
  (`SceneComponent.SetVisibility` `Slot target` _returnvalue_2 false)
  (set `PrimitiveComponent.bGenerateOverlapEvents` _returnvalue_2 `Slot target`))

(fn `SetSigns`
  (params (LeftSign :type String) (RightSign :type String))
  (bind _returnvalue (`KismetTextLibrary.Conv_StringToText` LeftSign))
  (bind _returnvalue_2 (`KismetTextLibrary.Conv_StringToText` RightSign))
  (`|ExecutionSequence`
    (:`then_0`
      (`TextRenderComponent.K2_SetText` (`self.LeftSignFront`) _returnvalue))
    (:`then_1`
      (`TextRenderComponent.K2_SetText` (`self.LeftSignBack`) _returnvalue))
    (:`then_2`
      (`TextRenderComponent.K2_SetText` (`self.RightSignFront`) _returnvalue_2))
    (:`then_3`
      (`TextRenderComponent.K2_SetText` (`self.RightSignBack`) _returnvalue_2))))

(fn `UserConstructionScript`)