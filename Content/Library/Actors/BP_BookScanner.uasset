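; BP_BookScanner is a grippable library scanner that detects red and blue books for a quest.
; When its Box overlaps a component, it searches the display name of that component's first material for "Red" or "Blue".
; A match plays a click sound and sends the matching scanned message to every widget implementing BPI_QuestBus.
; OnGrip stores the controller and grip information, and scanning does not require the scanner to be held.
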(event `VRGripInterface.OnGrip`
  (params (GrippingController :type "GripMotionControllerComponent Object Reference") (GripInformation :type "BPActorGripInformation Structure (by ref)"))
  (set `self.LMC` GrippingController)
  (set `self.Grip` GripInformation)
  (if (== (`self.IsHeld`) true)
    _))

(event `self.Box.OnComponentBeginOverlap`
  (params (OverlappedComponent :type "PrimitiveComponent Object Reference") (OtherActor :type "Actor Object Reference") (OtherComp :type "PrimitiveComponent Object Reference") (OtherBodyIndex :type Integer) (bFromSweep :type Boolean) (SweepResult :type "HitResult Structure (by ref)"))
  (if (`KismetStringLibrary.Contains` (`KismetSystemLibrary.GetDisplayName` (`PrimitiveComponent.GetMaterial` OtherComp 0)) "Red")
    (`GameplayStatics.PlaySound2D` "/Engine/VREditor/Sounds/UI/Click_on_Button_Cue.Click_on_Button_Cue" 1.0 1.0 0.0 null null)
    (bind _foundwidgets (`WidgetBlueprintLibrary.GetAllWidgetsWithInterface` "/Game/Library/Quest/BPI_QuestBus.BPI_QuestBus_C"))
    (for _array_element _foundwidgets
      (message `/Game/Library/Quest/BPI_QuestBus.RedBookScanned` _array_element))
    (elif (`KismetStringLibrary.Contains` (`KismetSystemLibrary.GetDisplayName` (`PrimitiveComponent.GetMaterial` OtherComp 0)) "Blue")
      (`GameplayStatics.PlaySound2D` "/Engine/VREditor/Sounds/UI/Click_on_Button_Cue.Click_on_Button_Cue" 1.0 1.0 0.0 null null)
      (bind _foundwidgets_2 (`WidgetBlueprintLibrary.GetAllWidgetsWithInterface` "/Game/Library/Quest/BPI_QuestBus.BPI_QuestBus_C"))
      (for _array_element_2 _foundwidgets_2
        (message `/Game/Library/Quest/BPI_QuestBus.BlueBookScanned` _array_element_2)))))

(fn `GetGripScripts`
  (returns (ArrayReference :type "Array of VRGripScriptBase Object Reference") (ReturnValue :type Boolean))
  (return _ false))

(fn `UserConstructionScript`)