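; BP_Bookbox is a book box actor that fills itself with BP_Book actors when play begins.
; A loop over Count spawns the books in two vertical stacks, splitting them at half the count.
; The stacks sit on either side of the static mesh along X, each book raised by a fixed step.
; Offsets use world axes, so the layout ignores the box's rotation.
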(event `self.ReceiveBeginPlay`
  (bind _count (`self.count`))
  (bind (_returnvalue_x _returnvalue_y _returnvalue_z) (`KismetMathLibrary.BreakVector` (`SceneComponent.K2_GetComponentLocation` (`self.StaticMesh`))))
  (bind (_returnvalue_x_2 _returnvalue_y_2 _returnvalue_z_2) (`KismetMathLibrary.BreakVector` (`SceneComponent.K2_GetComponentLocation` (`self.StaticMesh`))))
  (bind _returnvalue (/ _count 2))
  (for _index (range 1 (+ _count 1))
    (if (> _index _returnvalue)
      (`|SpawnActorFromClass` "/Game/Library/Actors/BP_Book.BP_Book_C" (`KismetMathLibrary.MakeTransform` (`KismetMathLibrary.MakeVector` (+ _returnvalue_x_2 11.0) _returnvalue_y_2 (- (+ _returnvalue_z_2 (* (- _index _returnvalue) 6)) 20.0)) (struct :`Yaw` 90.0)) "Undefined" "MultiplyWithRoot" null null)
      (else
        (`|SpawnActorFromClass` "/Game/Library/Actors/BP_Book.BP_Book_C" (`KismetMathLibrary.MakeTransform` (`KismetMathLibrary.MakeVector` (- _returnvalue_x 11.0) _returnvalue_y (- (+ _returnvalue_z (* _index 6.0)) 20.0)) (struct :`Yaw` 90.0)) "Undefined" "MultiplyWithRoot" null null)))))

(fn `UserConstructionScript`)