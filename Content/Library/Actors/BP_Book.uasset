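; BP_Book is a VR grippable book that locks into a book slot when placed, in the Library.
; On grip, it stores the gripping motion controller and grip information.
; When its mesh overlaps a component whose name contains "Book slot", it disables physics, makes the controller drop it and denies further gripping.
; It then snaps to the slot's location with a fixed rotation.
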(event `VRGripInterface.OnGrip`
  (params (GrippingController :type "GripMotionControllerComponent Object Reference") (GripInformation :type "BPActorGripInformation Structure (by ref)"))
  (set `self.LMC` GrippingController)
  (set `self.Grip` GripInformation))

(event `self.StaticMeshComponent.OnComponentBeginOverlap`
  (params (OverlappedComponent :type "PrimitiveComponent Object Reference") (OtherActor :type "Actor Object Reference") (OtherComp :type "PrimitiveComponent Object Reference") (OtherBodyIndex :type Integer) (bFromSweep :type Boolean) (SweepResult :type "HitResult Structure (by ref)"))
  (bind _returnvalue_location (`KismetMathLibrary.BreakTransform` (`SceneComponent.K2_GetComponentToWorld` OtherComp)))
  (if (`KismetStringLibrary.Contains` (`KismetSystemLibrary.GetObjectName` OtherComp) "Book slot")
    (`PrimitiveComponent.SetSimulatePhysics` (`self.StaticMeshComponent`) false)
    (`GripMotionControllerComponent.DropObjectByInterface` (`self.LMC`) self (`.GripID` (break `BPActorGripInformation` (`self.Grip`))) (0.0 0.0 0.0) (0.0 0.0 0.0))
    (`self.SetDenyGripping` self true)
    (`self.K2_SetActorLocationAndRotation` self _returnvalue_location (struct :`Pitch` 90.0) false false)))

(fn `GetGripScripts`
  (returns (ArrayReference :type "Array of VRGripScriptBase Object Reference") (ReturnValue :type Boolean))
  (return _ false))

(fn `UserConstructionScript`)